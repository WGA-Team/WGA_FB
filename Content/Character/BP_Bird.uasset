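; BP_Bird is the player bird in a Flappy Bird-style game, flapping upward when Jump is pressed by adding an upward acceleration force to its capsule.
; Each end of a capsule overlap tells BP_FB_GameMode to increment the score, add time-shift energy and adjust font and wall speeds.
; Any capsule hit shows the WBP_EndGame widget and pauses the game.
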(event OnComponentEndOverlap(CapsuleComponent)
  (params (OverlappedComponent :type Primitive%20Component%20Object%20Reference) (OtherActor :type Actor%20Object%20Reference) (OtherComp :type Primitive%20Component%20Object%20Reference) (OtherBodyIndex :type Integer))
  (bind _asbp_fb_game_mode (Utilities|Casting|CastToBP_FB_GameMode (Game|GetGameMode)))
  (Class|FlappyBirdsGameMode|IncrementScore _asbp_fb_game_mode)
  (Class|FlappyBirdsGameMode|AddTimeShiftEnergy _asbp_fb_game_mode)
  (Class|FlappyBirdsGameMode|IncrementSpeed _asbp_fb_game_mode -2.0 -1e+01))

(event OnComponentHit(CapsuleComponent)
  (params (HitComponent :type Primitive%20Component%20Object%20Reference) (OtherActor :type Actor%20Object%20Reference) (OtherComp :type Primitive%20Component%20Object%20Reference) (NormalImpulse :type Vector :default "0, 0, 0") (Hit :type Hit%20Result%20Structure%20%28by%20ref%29))
  (bind _returnvalue (UserInterface|CreateWidget "/Game/Widgets/WBP_EndGame.WBP_EndGame_C"))
  (UserInterface|Viewport|AddtoViewport _returnvalue 0)
  (Game|SetGamePaused true))

(event EventBeginPlay)

(event Collision|EventActorBeginOverlap
  (params (OtherActor :type Actor%20Object%20Reference)))

(event EventTick
  (params (DeltaSeconds :type Float%20%28single-precision%29)))

(event Input|ActionEvents|InputActionJump
  (params (Key :type Key%20Structure :default "None"))
  (:Pressed
    (Physics|AddForce (Variables|Default|GetCapsuleComponent) "0.000000,0.000000,50000.000000" "None" true)))

(fn ConstructionScript)