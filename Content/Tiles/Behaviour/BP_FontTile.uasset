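; Scenery tile that fills itself with randomised decoration and scrolls along X during play.
; On BeginPlay it calls PlaceActors for tree, mountain and cloud Blueprints, each with its own count range, spawn area and scale limits, keeping clouds in a higher band.
; Each Tick it offsets the Font component's relative X by the game mode's font speed times delta time and applies that as the actor's relative location.
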(event EventBeginPlay
  (Class|FontTile|PlaceActors self "/Game/Tiles/FontActors/BP_Tree_01.BP_Tree_01_C" 2 5 "-850.000000,10.000000,-580.000000" "850.000000,10.000000,-250.000000" 0.2 0.5)
  (Class|FontTile|PlaceActors "/Game/Tiles/FontActors/BP_Tree_02.BP_Tree_02_C" 2 5 "-900.000000,10.000000,-600.000000" "900.000000,10.000000,-250.000000" 0.2 0.5)
  (Class|FontTile|PlaceActors "/Game/Tiles/FontActors/BP_Tree_03.BP_Tree_03_C" 2 5 "-850.000000,10.000000,-530.000000" "850.000000,10.000000,-460.000000" 0.2 0.5)
  (Class|FontTile|PlaceActors "/Game/Tiles/FontActors/BP_Tree_04.BP_Tree_04_C" 2 5 "-900.000000,10.000000,-580.000000" "900.000000,10.000000,-250.000000" 0.2 0.5)
  (Class|FontTile|PlaceActors "/Game/Tiles/FontActors/BP_Mountains_01.BP_Mountains_01_C" 1 2 "-900.000000,10.000000,-600.000000" "900.000000,10.000000,-300.000000" 0.5 1.0)
  (Class|FontTile|PlaceActors "/Game/Tiles/FontActors/BP_Mountains_02.BP_Mountains_02_C" 1 2 "-900.000000,10.000000,-600.000000" "900.000000,10.000000,-300.000000" 0.5 1.0)
  (Class|FontTile|PlaceActors "/Game/Tiles/FontActors/BP_Cloud_01.BP_Cloud_01_C" 1 4 "-900.000000,5.000000,40.000000" "900.000000,5.000000,500.000000" 0.5 1.0)
  (Class|FontTile|PlaceActors "/Game/Tiles/FontActors/BP_Cloud_02.BP_Cloud_02_C" 1 4 "-900.000000,5.000000,40.000000" "900.000000,5.000000,500.000000" 0.5 1.0))

(event Collision|EventActorBeginOverlap
  (params (OtherActor :type Actor%20Object%20Reference)))

(event EventTick
  (params (DeltaSeconds :type Float%20%28single-precision%29))
  (bind _font (Variables|Default|GetFont))
  (bind _returnvalue (Transformation|GetRelativeTransform _font))
  (bind _asbp_fb_game_mode (Utilities|Casting|CastToBP_FB_GameMode (Game|GetGameMode)))
  (bind _returnvalue_2 (Class|FlappyBirdsGameMode|GetFontSpeed _asbp_fb_game_mode))
  (Transformation|SetActorRelativeLocation (Math|Vector|MakeVector (+ (* _returnvalue_2 DeltaSeconds) (.x (.location _returnvalue))) (.y (.location _returnvalue)) (.z (.location _returnvalue)))))

(fn ConstructionScript)